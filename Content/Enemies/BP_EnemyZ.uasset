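; BP_EnemyZ is an enemy Blueprint that sets a zigzag movement direction, building on a parent class.
; A looping timer started on BeginPlay flips a sign every ZigInterval.
; Each flip rebuilds MovementVector from the actor's right vector plus its forward vector scaled by signed ZigStrength, so the zigzag swings along the forward axis.
; The file only sets this vector and does not apply the movement itself.
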(event `self.ReceiveBeginPlay`
  (`parent.ReceiveBeginPlay`)
  (set `self.ZigSign` 1.0)
  (`KismetSystemLibrary.K2_SetTimerDelegate` (delegate `FlipZig`) (`self.ZigInterval`) true))

(event `FlipZig`
  (set `self.ZigSign` (* (`self.ZigSign`) -1.0))
  (set `self.MovementVector` (+ (* (`self.GetActorForwardVector`) (* (`self.ZigStrength`) (`self.ZigSign`))) (`self.GetActorRightVector`))))

(fn `UserConstructionScript`
  (`parent.UserConstructionScript`))