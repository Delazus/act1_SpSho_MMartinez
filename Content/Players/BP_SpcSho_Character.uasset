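; Player spaceship character for a shooter: moves, banks, fires, shields itself and tracks lives.
; Enhanced Input drives movement, and Tick interpolates the ship mesh's roll toward a tilt set by horizontal input.
; Firing spawns ammo at FirePoint, with a timer limiting the rate.
; A timed shield shows its mesh and blocks DamageActor, which otherwise removes a life and calls PlayerDead on the game mode at zero.
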(event `self.ReceiveBeginPlay`
  ; Setup Enhanched Input
  (bind _asplayer_controller (cast `PlayerController` (`self.GetController`)))
  (bind _returnvalue (pcsubsystem `EnhancedInputLocalPlayerSubsystem` _asplayer_controller))
  (`/Engine/EditorBlueprintResources/StandardMacros.IsValid` _returnvalue
    (:`Is Valid`
      (`EnhancedInputSubsystemInterface.AddMappingContext` _returnvalue "/Game/Input/BP_InputMapping.BP_InputMapping" 0 (struct))
      (`self.Soun Ambient`)
      (set `self.BaseMeshRotation` (`SceneComponent.RelativeRotation` (`self.SM_StarSparrow18`))))))

(event `self.ReceiveTick`
  (params (DeltaSeconds :type "Float (single-precision)"))
  (set `self.CurrentTilt` (`KismetMathLibrary.FInterpTo` (`self.CurrentTilt`) (`self.TargetTilt`) DeltaSeconds (`self.TiltSpeed`)))
  (`SceneComponent.K2_SetRelativeRotation` (`self.SM_StarSparrow18`) (`KismetMathLibrary.MakeRotator` (+ (.roll (`self.BaseMeshRotation`)) (`self.CurrentTilt`)) (.pitch (`self.BaseMeshRotation`)) (.yaw (`self.BaseMeshRotation`))) false false))

(event `EnhancedInput|/Game/Input/BP_InputMove`
  (params (ActionValue :type "Vector2D Structure") (ElapsedSeconds :type "Float (double-precision)") (TriggeredSeconds :type "Float (double-precision)") (InputAction :type "InputAction Object Reference" :default "/Game/Input/BP_InputMove.BP_InputMove"))
  (:`Triggered`
    (`self.AddMovementInput` (`self.GetActorRightVector`) ActionValue_X)
    (`self.AddMovementInput` (`self.GetActorForwardVector`) ActionValue_Y)
    (set `self.TargetTilt` (* ActionValue_X (`self.MaxTilt`))))
  (:`Completed`
    (set `self.TargetTilt` 0.0)))

(event `EnhancedInput|/Game/Input/BP_InputFire`
  (params (ActionValue :type Boolean) (ElapsedSeconds :type "Float (double-precision)") (TriggeredSeconds :type "Float (double-precision)") (InputAction :type "InputAction Object Reference" :default "/Game/Input/BP_InputFire.BP_InputFire"))
  (:`Triggered`
    (if (`self.CanFire`)
      (`self.DoFire_OneBullet`)
      (`GameplayStatics.PlaySound2D` "/Game/Sounds/Sci-Fi_Gun_1-1_Cue.Sci-Fi_Gun_1-1_Cue" 1.0 1.0 0.0 null null)
      (set `self.CanFire` false)
      (`KismetSystemLibrary.K2_SetTimerDelegate` (delegate `UpdateFire`) (`self.FireDelay`)))))

(event `UpdateFire`
  (set `self.CanFire` true))

(event `DamageActor`
  (if (not (`self.ShieldActive`))
    (bind _output_get (set `self.LifesPlayer` (- (`self.LifesPlayer`) 1)))
    (if (<= _output_get 0)
      (bind _asbp_sp_sho_play_mode (cast `/Game/BP_SpSho_PlayMode` (`GameplayStatics.GetGameMode`)))
      (`/Game/BP_SpSho_PlayMode.PlayerDead` _asbp_sp_sho_play_mode))))

(event `ActiveShield`
  (if (not (`self.ShieldActive`))
    (set `self.ShieldActive` true)
    (`SceneComponent.SetVisibility` (`self.ShieldMesh`) true true)
    (`KismetSystemLibrary.Delay` (`self.ShieldDuration`))
    (set `self.ShieldActive` false)
    (`SceneComponent.SetVisibility` (`self.ShieldMesh`) false false)))

(event `EnhancedInput|/Game/Input/BP_InputShield`
  (params (ActionValue :type Boolean) (ElapsedSeconds :type "Float (double-precision)") (TriggeredSeconds :type "Float (double-precision)") (InputAction :type "InputAction Object Reference" :default "/Game/Input/BP_InputShield.BP_InputShield"))
  (:`Triggered`
    (`self.ActiveShield`)))

(event `Soun Ambient`
  (`GameplayStatics.PlaySound2D` "/Game/Sounds/Ambient.Ambient" 0.1 1.0 0.0 null null))

(fn `DoFire_OneBullet`
  (`|SpawnActorFromClass` (`self.Ammo`) (`SceneComponent.K2_GetComponentToWorld` (`self.FirePoint`)) "Undefined" "MultiplyWithRoot" null null))

(fn `UserConstructionScript`)